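; Auto-walking puzzle character that navigates BP_CubeBase paths, collecting keys and click-reset items, unlocking goals, and creating the HUD and music.
; Tick moves it forward or applies flagged 90/180-degree turns.
; Front and side overlap boxes read cube type, layer and state to set those flags and snap position, with IsClockwise choosing the side probe.
; Yaw comparisons against stair cubes decide stair entry, which shifts PlayerLayer up or down.
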(event OnComponentEndOverlap(BoxBegin)
  (params (OverlappedComponent :type Primitive%20Component%20Object%20Reference) (OtherActor :type Actor%20Object%20Reference) (OtherComp :type Primitive%20Component%20Object%20Reference) (OtherBodyIndex :type Integer))
  (bind _asbp_cube_base (Utilities|Casting|CastToBP_CubeBase OtherActor))
  (if (== (Actor|GetComponentbyClass _asbp_cube_base "/Script/Engine.BoxComponent") OtherComp)
    (if (== (Variables|/Game/Hou/BluePrints/BP_CubeBase.BP_CubeBase_C|GetCubeLayer _asbp_cube_base) (Variables|Default|GetPlayerLayer))
      (switch int (Variables|/Game/Hou/BluePrints/BP_CubeBase.BP_CubeBase_C|GetCubeType _asbp_cube_base)
        (:2
          (Variables|Default|SetIsRightAngle true)
          (Variables|Default|SetIsRotateL true)
          (Transformation|SetActorLocation (Math|Vector|MakeVector (.X (Math|Vector|BreakVector (Transformation|GetActorLocation _asbp_cube_base))) (.Y (Math|Vector|BreakVector (Transformation|GetActorLocation _asbp_cube_base))) (.Z (Math|Vector|BreakVector (Transformation|GetActorLocation)))) false false :!label _label))
        (:6
          (Variables|Default|SetRotating false :!label _label_2))
        (:7
          (Variables|Default|SetIsClockwise (not (Variables|Default|GetIsClockwise)))
          (Variables|Default|SetRotate360 true)
          (goto _label)))
      (else
        (switch int (Variables|/Game/Hou/BluePrints/BP_CubeBase.BP_CubeBase_C|GetCubeType _asbp_cube_base)
          (:6
            (goto _label_2)))))))

(event OnComponentBeginOverlap(BoxBegin)
  (params (OverlappedComponent :type Primitive%20Component%20Object%20Reference) (OtherActor :type Actor%20Object%20Reference) (OtherComp :type Primitive%20Component%20Object%20Reference) (OtherBodyIndex :type Integer) (bFromSweep :type Boolean) (SweepResult :type Hit%20Result%20Structure%20%28by%20ref%29))
  (bind _asbp_cube_base (Utilities|Casting|CastToBP_CubeBase OtherActor))
  (if (== (Actor|GetComponentbyClass _asbp_cube_base "/Script/Engine.BoxComponent") OtherComp)
    ;[1 1 1] HeightCube
    (if (== (Variables|/Game/Hou/BluePrints/BP_CubeBase.BP_CubeBase_C|GetCubeLayer _asbp_cube_base) (Variables|Default|GetPlayerLayer))
      (if (Variables|/Game/Hou/BluePrints/BP_CubeBase.BP_CubeBase_C|GetHaveTop _asbp_cube_base)
        ;[1 1 1] 楼梯中的判断，360旋转
        (if (Variables|Default|GetIsStair)
          (if (not (Variables|/Game/Hou/BluePrints/BP_CubeBase.BP_CubeBase_C|GetTopIsStair _asbp_cube_base))
            (Variables|Default|SetRotate360 true :!label _label)
            (if (Variables|Default|GetUpStair)
              (bind _result (Math|Integer|DecrementInt (Variables|Default|GetPlayerLayer))
                (:%20%20
                  (Variables|Default|SetPlayerLayer _result)
                  (Variables|Default|SetRotating true :!label _label_2)))
              (elif (Variables|Default|GetDownStair)
                (bind _result_2 (Math|Integer|IncrementInt (Variables|Default|GetPlayerLayer))
                  (:%20%20
                    (Variables|Default|SetPlayerLayer _result_2)
                    (goto _label_2))))))
          (elif (not (Variables|/Game/Hou/BluePrints/BP_CubeBase.BP_CubeBase_C|GetTopIsStair _asbp_cube_base))
            ;[1 1 1] Memory
            (if (not (Variables|Default|GetIsRotateL)) :!label _label_3
              (Variables|Default|SetIsRotateF true)
              (Variables|Default|SetRotating true)
              (Transformation|SetActorLocation (- (Math|Vector|MakeVector (.X (Math|Vector|BreakVector (Transformation|GetActorLocation _asbp_cube_base))) (.Y (Math|Vector|BreakVector (Transformation|GetActorLocation _asbp_cube_base))) (.Z (Math|Vector|BreakVector (Transformation|GetActorLocation)))) (* (Transformation|GetActorForwardVector) (Math|Vector|MakeVector 1e+02 1e+02 0.0))) false false))))
        (else
          (switch int (Variables|/Game/Hou/BluePrints/BP_CubeBase.BP_CubeBase_C|GetCubeType _asbp_cube_base)
            (:0
              (Variables|/Game/Hou/BluePrints/BP_CubeBase.BP_CubeBase_C|SetIsPlayer _asbp_cube_base true)
              (if (not (Variables|/Game/Hou/BluePrints/BP_CubeBase.BP_CubeBase_C|GetIsActive _asbp_cube_base)) :!label _label_4
                (if (Variables|Default|GetIsStair) :!label _label_5
                  (goto _label)
                  (else
                    (goto _label_3)))))
            (:1
              (goto _label_5))
            (:2
              (Variables|/Game/Hou/BluePrints/BP_CubeBase.BP_CubeBase_C|SetIsPlayer _asbp_cube_base true :!label _label_6))
            (:3
              ;[1 1 1] Iteam
              (bind _asbp_cube_reset_click (Utilities|Casting|CastToBP_CubeResetClick OtherActor))
              (if (Variables|/Game/Hou/BluePrints/BP_CubeResetClick.BP_CubeResetClick_C|GetIsIteam _asbp_cube_reset_click)
                (bind _aspuzzle_player_controller (Utilities|Casting|CastToPuzzlePlayerController (Class|GameplayStatics|GetPlayerControllerfromID)))
                (Variables|/Game/PuzzleBP/Blueprints/PuzzlePlayerController.PuzzlePlayerController_C|SetClickCount _aspuzzle_player_controller 0)
                (Variables|/Game/Hou/BluePrints/BP_CubeResetClick.BP_CubeResetClick_C|SetIsIteam _asbp_cube_reset_click false)
                (Rendering|SetVisibility (Variables|/Game/Hou/BluePrints/BP_CubeResetClick.BP_CubeResetClick_C|GetSphere _asbp_cube_reset_click) false false)
                (goto _label_4)
                (else
                  (goto _label_4))))
            (:4
              ;[1 1 1] Goal
              (bind _asbp_cube_goal (Utilities|Casting|CastToBP_CubeGoal OtherActor))
              (if (Variables|Default|GetIsKey)
                (Variables|/Game/Hou/BluePrints/BP_CubeGoal.BP_CubeGoal_C|SetSwitchOn _asbp_cube_goal true)
                (Collision|SetCollisionEnabled (Variables|/Game/Hou/BluePrints/BP_CubeGoal.BP_CubeGoal_C|GetCube1 _asbp_cube_goal) "QueryAndPhysics")
                (else
                  (goto _label_5))))
            (:5
              ;[1 1 1] Key
              (bind _asbp_cube_key (Utilities|Casting|CastToBP_CubeKey OtherActor))
              (if (Variables|/Game/Hou/BluePrints/BP_CubeKey.BP_CubeKey_C|GetIsIteam _asbp_cube_key)
                (Variables|Default|SetIsKey true)
                (Variables|/Game/Hou/BluePrints/BP_CubeKey.BP_CubeKey_C|SetIsIteam _asbp_cube_key false)
                (Rendering|SetVisibility (Variables|/Game/Hou/BluePrints/BP_CubeKey.BP_CubeKey_C|GetCone _asbp_cube_key) false false)
                (goto _label_4)
                (else
                  (goto _label_4))))
            (:6
              ;[1 1 1] Stair
              (Variables|/Game/Hou/BluePrints/BP_CubeBase.BP_CubeBase_C|SetIsPlayer _asbp_cube_base true)
              (Development|PrintString (Utilities|String|ToString(Float) (- (.Yaw (Math|Vector|GetYawPitchfromVector (Math|Rotator|GetRotationXVector (Transformation|GetActorRotation)))) (.Yaw (Math|Vector|GetYawPitchfromVector (Math|Rotator|GetRotationXVector (Transformation|GetActorRotation _asbp_cube_base)))))))
              ;;[1 1 1] 上
              (if (<= (- (.Yaw (Math|Vector|GetYawPitchfromVector (Math|Rotator|GetRotationXVector (Transformation|GetActorRotation)))) (.Yaw (Math|Vector|GetYawPitchfromVector (Math|Rotator|GetRotationXVector (Transformation|GetActorRotation _asbp_cube_base))))) 0.1)
                (if (> (- (.Yaw (Math|Vector|GetYawPitchfromVector (Math|Rotator|GetRotationXVector (Transformation|GetActorRotation)))) (.Yaw (Math|Vector|GetYawPitchfromVector (Math|Rotator|GetRotationXVector (Transformation|GetActorRotation _asbp_cube_base))))) -0.1)
                  (if (not (Variables|Default|GetIsStair)) :!label _label_7
                    (if (== (Variables|/Game/Hou/BluePrints/BP_CubeBase.BP_CubeBase_C|GetCubeLayer _asbp_cube_base) (Variables|Default|GetPlayerLayer))
                      (bind _result_3 (Math|Integer|IncrementInt (Variables|Default|GetPlayerLayer))
                        (:%20%20
                          (bind _output_get (Variables|Default|SetPlayerLayer _result_3))
                          (Variables|Default|SetUpStair true)))
                      (else
                        (bind _result_4 (Math|Integer|DecrementInt (Variables|Default|GetPlayerLayer))
                          (:%20%20
                            (bind _output_get_2 (Variables|Default|SetPlayerLayer _result_4))
                            (Variables|Default|SetDownStair true)))))
                    (Variables|Default|SetIsStair true)
                    (Variables|Default|SetRotating true))
                  (else
                    (if (<= (- (.Yaw (Math|Vector|GetYawPitchfromVector (Math|Rotator|GetRotationXVector (Transformation|GetActorRotation)))) (.Yaw (Math|Vector|GetYawPitchfromVector (Math|Rotator|GetRotationXVector (Transformation|GetActorRotation _asbp_cube_base))))) 360.100006) :!label _label_8
                      (if (> (- (.Yaw (Math|Vector|GetYawPitchfromVector (Math|Rotator|GetRotationXVector (Transformation|GetActorRotation)))) (.Yaw (Math|Vector|GetYawPitchfromVector (Math|Rotator|GetRotationXVector (Transformation|GetActorRotation _asbp_cube_base))))) 359.899994)
                        (goto _label_7)
                        (else
                          _)))
                    (if (not (Variables|Default|GetIsStair)) :!label _label_9
                      (goto _label_3))))
                (else
                  (goto _label_8))))
            (:7
              (goto _label_6)))))
      (elif (Variables|/Game/Hou/BluePrints/BP_CubeBase.BP_CubeBase_C|GetIsActive _asbp_cube_base)
        (switch int (Variables|/Game/Hou/BluePrints/BP_CubeBase.BP_CubeBase_C|GetCubeType _asbp_cube_base)
          (:6
            (Variables|/Game/Hou/BluePrints/BP_CubeBase.BP_CubeBase_C|SetIsPlayer _asbp_cube_base true)
            ;;[1 1 1] 下
            (if (<= (- (.Yaw (Math|Vector|GetYawPitchfromVector (Math|Rotator|GetRotationXVector (Transformation|GetActorRotation)))) (.Yaw (Math|Vector|GetYawPitchfromVector (Math|Rotator|GetRotationXVector (Transformation|GetActorRotation _asbp_cube_base))))) -179.899994)
              (if (> (- (.Yaw (Math|Vector|GetYawPitchfromVector (Math|Rotator|GetRotationXVector (Transformation|GetActorRotation)))) (.Yaw (Math|Vector|GetYawPitchfromVector (Math|Rotator|GetRotationXVector (Transformation|GetActorRotation _asbp_cube_base))))) -180.100006)
                (goto _label_7)
                (else
                  _)))
            (if (<= (- (.Yaw (Math|Vector|GetYawPitchfromVector (Math|Rotator|GetRotationXVector (Transformation|GetActorRotation)))) (.Yaw (Math|Vector|GetYawPitchfromVector (Math|Rotator|GetRotationXVector (Transformation|GetActorRotation _asbp_cube_base))))) 180.100006)
              (if (> (- (.Yaw (Math|Vector|GetYawPitchfromVector (Math|Rotator|GetRotationXVector (Transformation|GetActorRotation)))) (.Yaw (Math|Vector|GetYawPitchfromVector (Math|Rotator|GetRotationXVector (Transformation|GetActorRotation _asbp_cube_base))))) 179.899994)
                (goto _label_7)
                (else
                  (goto _label_9)))
              (else
                (goto _label_9)))))))))

(event OnComponentEndOverlap(Box1)
  (params (OverlappedComponent :type Primitive%20Component%20Object%20Reference) (OtherActor :type Actor%20Object%20Reference) (OtherComp :type Primitive%20Component%20Object%20Reference) (OtherBodyIndex :type Integer))
  (bind _playerlayer (Variables|Default|GetPlayerLayer))
  (if (Variables|Default|GetIsClockwise)
    (bind _asbp_cube_base (Utilities|Casting|CastToBP_CubeBase OtherActor))
    (if (== (Actor|GetComponentbyClass _asbp_cube_base "/Script/Engine.BoxComponent") OtherComp)
      ;[1 1 1] HeightCube
      (if (== (Variables|/Game/Hou/BluePrints/BP_CubeBase.BP_CubeBase_C|GetCubeLayer _asbp_cube_base) _playerlayer)
        (switch int (Variables|/Game/Hou/BluePrints/BP_CubeBase.BP_CubeBase_C|GetCubeType _asbp_cube_base))
        (elif (> (Variables|/Game/Hou/BluePrints/BP_CubeBase.BP_CubeBase_C|GetCubeLayer _asbp_cube_base) _playerlayer)
          _)))))

(event OnComponentEndOverlap(BoxEnd)
  (params (OverlappedComponent :type Primitive%20Component%20Object%20Reference) (OtherActor :type Actor%20Object%20Reference) (OtherComp :type Primitive%20Component%20Object%20Reference) (OtherBodyIndex :type Integer))
  (bind _asbp_cube_base (Utilities|Casting|CastToBP_CubeBase OtherActor))
  (if (== (Actor|GetComponentbyClass _asbp_cube_base "/Script/Engine.BoxComponent") OtherComp)
    (if (== (Variables|/Game/Hou/BluePrints/BP_CubeBase.BP_CubeBase_C|GetCubeLayer _asbp_cube_base) (Variables|Default|GetPlayerLayer))
      (switch int (Variables|/Game/Hou/BluePrints/BP_CubeBase.BP_CubeBase_C|GetCubeType _asbp_cube_base)
        (:0
          (Variables|/Game/Hou/BluePrints/BP_CubeBase.BP_CubeBase_C|SetIsPlayer _asbp_cube_base false :!label _label))
        (:2
          (goto _label))
        (:6
          ;[1 1 1] HeightCube
          (Variables|Default|SetIsStair false :!label _label_2)
          (Variables|Default|SetUpStair false)
          (Variables|Default|SetDownStair false)
          (goto _label))
        (:7
          (goto _label))
        (:8
          (bind _asbp_cube_timer (Utilities|Casting|CastToBP_CubeTimer _asbp_cube_base))
          (bind _result (Math|Integer|DecrementInt (Variables|/Game/Hou/BluePrints/BP_CubeTimer.BP_CubeTimer_C|GetDisappearCount _asbp_cube_timer))
            (:%20%20
              (Variables|/Game/Hou/BluePrints/BP_CubeTimer.BP_CubeTimer_C|SetDisappearCount _asbp_cube_timer _result)))))
      (else
        (switch int (Variables|/Game/Hou/BluePrints/BP_CubeBase.BP_CubeBase_C|GetCubeType _asbp_cube_base)
          (:0
            (goto _label))
          (:2
            (goto _label))
          (:6
            (goto _label_2))
          (:7
            (goto _label)))))))

(event OnComponentBeginOverlap(Box1)
  (params (OverlappedComponent :type Primitive%20Component%20Object%20Reference) (OtherActor :type Actor%20Object%20Reference) (OtherComp :type Primitive%20Component%20Object%20Reference) (OtherBodyIndex :type Integer) (bFromSweep :type Boolean) (SweepResult :type Hit%20Result%20Structure%20%28by%20ref%29))
  (if (Variables|Default|GetIsClockwise)
    (if (not (Variables|Default|GetIsRightAngle))
      (bind _asbp_cube_base (Utilities|Casting|CastToBP_CubeBase OtherActor))
      (if (== (Actor|GetComponentbyClass _asbp_cube_base "/Script/Engine.BoxComponent") OtherComp)
        ;[1 1 1] HeightCube
        (if (== (Variables|/Game/Hou/BluePrints/BP_CubeBase.BP_CubeBase_C|GetCubeLayer _asbp_cube_base) (Variables|Default|GetPlayerLayer))
          (if (Variables|/Game/Hou/BluePrints/BP_CubeBase.BP_CubeBase_C|GetHaveTop _asbp_cube_base)
            (if (not (Variables|/Game/Hou/BluePrints/BP_CubeBase.BP_CubeBase_C|GetTopIsStair _asbp_cube_base))
              (Variables|Default|SetRotating false :!label _label))
            (else
              (switch int (Variables|/Game/Hou/BluePrints/BP_CubeBase.BP_CubeBase_C|GetCubeType _asbp_cube_base)
                (:0
                  ;[1 1 1] Memory
                  (if (Variables|/Game/Hou/BluePrints/BP_CubeBase.BP_CubeBase_C|GetIsActive _asbp_cube_base) :!label _label_2
                    (if (Variables|Default|GetRotating) :!label _label_3
                      (if (not (Variables|Default|GetIsStair))
                        (if (not (Variables|Default|GetIsRotateL)) :!label _label_4
                          (Variables|Default|SetIsRotateL true)
                          (Variables|Default|SetRotating true)
                          (Transformation|SetActorLocation (- (Math|Vector|MakeVector (.X (Math|Vector|BreakVector (Transformation|GetActorLocation _asbp_cube_base))) (.Y (Math|Vector|BreakVector (Transformation|GetActorLocation _asbp_cube_base))) (.Z (Math|Vector|BreakVector (Transformation|GetActorLocation)))) (* (* (Transformation|GetActorRightVector) -1) (Math|Vector|MakeVector 1e+02 1e+02 0.0))) false false)))
                      (else
                        (goto _label_4)))
                    (else
                      (goto _label))))
                (:1
                  (goto _label))
                (:2
                  (goto _label_2))
                (:3
                  ;[1 1 1] iteam
                  (bind _asbp_cube_reset_click (Utilities|Casting|CastToBP_CubeResetClick OtherActor))
                  (if (Variables|/Game/Hou/BluePrints/BP_CubeResetClick.BP_CubeResetClick_C|GetIsIteam _asbp_cube_reset_click)
                    (bind _aspuzzle_player_controller (Utilities|Casting|CastToPuzzlePlayerController (Class|GameplayStatics|GetPlayerControllerfromID)))
                    (Variables|/Game/PuzzleBP/Blueprints/PuzzlePlayerController.PuzzlePlayerController_C|SetClickCount _aspuzzle_player_controller 0)
                    (Variables|/Game/Hou/BluePrints/BP_CubeResetClick.BP_CubeResetClick_C|SetIsIteam _asbp_cube_reset_click false)
                    (Rendering|SetVisibility (Variables|/Game/Hou/BluePrints/BP_CubeResetClick.BP_CubeResetClick_C|GetSphere _asbp_cube_reset_click) false false)
                    (goto _label_2)
                    (else
                      (goto _label_2))))
                (:4
                  ;[1 1 1] Goal
                  (bind _asbp_cube_goal (Utilities|Casting|CastToBP_CubeGoal OtherActor))
                  (if (Variables|Default|GetIsKey)
                    (Variables|/Game/Hou/BluePrints/BP_CubeGoal.BP_CubeGoal_C|SetSwitchOn _asbp_cube_goal true)
                    (Collision|SetCollisionEnabled (Variables|/Game/Hou/BluePrints/BP_CubeGoal.BP_CubeGoal_C|GetCube1 _asbp_cube_goal) "QueryAndPhysics")
                    (goto _label_3)
                    (else
                      (goto _label))))
                (:5
                  ;[1 1 1] Key
                  (bind _asbp_cube_key (Utilities|Casting|CastToBP_CubeKey OtherActor))
                  (if (Variables|/Game/Hou/BluePrints/BP_CubeKey.BP_CubeKey_C|GetIsIteam _asbp_cube_key)
                    (Variables|Default|SetIsKey true)
                    (Variables|/Game/Hou/BluePrints/BP_CubeKey.BP_CubeKey_C|SetIsIteam _asbp_cube_key false)
                    (Rendering|SetVisibility (Variables|/Game/Hou/BluePrints/BP_CubeKey.BP_CubeKey_C|GetCone _asbp_cube_key) false false)
                    (goto _label_2)
                    (else
                      (goto _label_2))))
                (:6
                  ;[1 1 1] Stair
                  ;;[1 1 1] 上
                  (if (<= (- (.Yaw (Math|Vector|GetYawPitchfromVector (Math|Rotator|GetRotationXVector (Transformation|GetActorRotation)))) (.Yaw (Math|Vector|GetYawPitchfromVector (Math|Rotator|GetRotationXVector (Transformation|GetActorRotation _asbp_cube_base))))) -269.899994)
                    (if (> (- (.Yaw (Math|Vector|GetYawPitchfromVector (Math|Rotator|GetRotationXVector (Transformation|GetActorRotation)))) (.Yaw (Math|Vector|GetYawPitchfromVector (Math|Rotator|GetRotationXVector (Transformation|GetActorRotation _asbp_cube_base))))) -270.100006)
                      _
                      (else
                        (if (<= (- (.Yaw (Math|Vector|GetYawPitchfromVector (Math|Rotator|GetRotationXVector (Transformation|GetActorRotation)))) (.Yaw (Math|Vector|GetYawPitchfromVector (Math|Rotator|GetRotationXVector (Transformation|GetActorRotation _asbp_cube_base))))) 90.099998) :!label _label_5
                          (if (> (- (.Yaw (Math|Vector|GetYawPitchfromVector (Math|Rotator|GetRotationXVector (Transformation|GetActorRotation)))) (.Yaw (Math|Vector|GetYawPitchfromVector (Math|Rotator|GetRotationXVector (Transformation|GetActorRotation _asbp_cube_base))))) 89.900002)
                            _
                            (else
                              (goto _label)))
                          (else
                            (goto _label)))))
                    (else
                      (goto _label_5)))
                  (Variables|Default|SetRotating true)
                  (Variables|Default|SetIsRotateL true :!label _label_6))
                (:7
                  (goto _label_2))
                (:8
                  (goto _label_2)))))
          (elif (Variables|/Game/Hou/BluePrints/BP_CubeBase.BP_CubeBase_C|GetIsActive _asbp_cube_base)
            (switch int (Variables|/Game/Hou/BluePrints/BP_CubeBase.BP_CubeBase_C|GetCubeType _asbp_cube_base)
              (:6
                ;;[1 1 1] 下
                (if (<= (- (.Yaw (Math|Vector|GetYawPitchfromVector (Math|Rotator|GetRotationXVector (Transformation|GetActorRotation)))) (.Yaw (Math|Vector|GetYawPitchfromVector (Math|Rotator|GetRotationXVector (Transformation|GetActorRotation _asbp_cube_base))))) -89.900002)
                  (if (> (- (.Yaw (Math|Vector|GetYawPitchfromVector (Math|Rotator|GetRotationXVector (Transformation|GetActorRotation)))) (.Yaw (Math|Vector|GetYawPitchfromVector (Math|Rotator|GetRotationXVector (Transformation|GetActorRotation _asbp_cube_base))))) -90.099998)
                    _
                    (else
                      (if (<= (- (.Yaw (Math|Vector|GetYawPitchfromVector (Math|Rotator|GetRotationXVector (Transformation|GetActorRotation)))) (.Yaw (Math|Vector|GetYawPitchfromVector (Math|Rotator|GetRotationXVector (Transformation|GetActorRotation _asbp_cube_base))))) 270.100006) :!label _label_7
                        (if (> (- (.Yaw (Math|Vector|GetYawPitchfromVector (Math|Rotator|GetRotationXVector (Transformation|GetActorRotation)))) (.Yaw (Math|Vector|GetYawPitchfromVector (Math|Rotator|GetRotationXVector (Transformation|GetActorRotation _asbp_cube_base))))) 269.899994)
                          _
                          (else
                            (goto _label)))
                        (else
                          (goto _label)))))
                  (else
                    (goto _label_7)))
                (Variables|Default|SetRotating false)
                (goto _label_6)))))))))

(event OnComponentBeginOverlap(Box2)
  (params (OverlappedComponent :type Primitive%20Component%20Object%20Reference) (OtherActor :type Actor%20Object%20Reference) (OtherComp :type Primitive%20Component%20Object%20Reference) (OtherBodyIndex :type Integer) (bFromSweep :type Boolean) (SweepResult :type Hit%20Result%20Structure%20%28by%20ref%29))
  (if (not (Variables|Default|GetIsClockwise))
    (if (not (Variables|Default|GetIsRightAngle))
      (bind _asbp_cube_base (Utilities|Casting|CastToBP_CubeBase OtherActor))
      (if (== (Actor|GetComponentbyClass _asbp_cube_base "/Script/Engine.BoxComponent") OtherComp)
        ;[1 1 1] HeightCube
        (if (== (Variables|/Game/Hou/BluePrints/BP_CubeBase.BP_CubeBase_C|GetCubeLayer _asbp_cube_base) (Variables|Default|GetPlayerLayer))
          (if (Variables|/Game/Hou/BluePrints/BP_CubeBase.BP_CubeBase_C|GetHaveTop _asbp_cube_base)
            (if (not (Variables|/Game/Hou/BluePrints/BP_CubeBase.BP_CubeBase_C|GetTopIsStair _asbp_cube_base))
              (Variables|Default|SetRotating false :!label _label))
            (else
              (switch int (Variables|/Game/Hou/BluePrints/BP_CubeBase.BP_CubeBase_C|GetCubeType _asbp_cube_base)
                (:0
                  ;[1 1 1] Memory
                  (if (Variables|/Game/Hou/BluePrints/BP_CubeBase.BP_CubeBase_C|GetIsActive _asbp_cube_base) :!label _label_2
                    (if (Variables|Default|GetRotating) :!label _label_3
                      (if (not (Variables|Default|GetIsStair))
                        (if (not (Variables|Default|GetIsRotateL)) :!label _label_4
                          (Variables|Default|SetIsRotateL true)
                          (Variables|Default|SetRotating true)
                          (Transformation|SetActorLocation (- (Math|Vector|MakeVector (.X (Math|Vector|BreakVector (Transformation|GetActorLocation _asbp_cube_base))) (.Y (Math|Vector|BreakVector (Transformation|GetActorLocation _asbp_cube_base))) (.Z (Math|Vector|BreakVector (Transformation|GetActorLocation)))) (* (* (Transformation|GetActorRightVector) -1) (Math|Vector|MakeVector -1e+02 -1e+02 0.0))) false false)))
                      (else
                        (goto _label_4)))
                    (else
                      (goto _label))))
                (:1
                  (goto _label))
                (:2
                  (goto _label_2))
                (:3
                  ;[1 1 1] iteam
                  (bind _asbp_cube_reset_click (Utilities|Casting|CastToBP_CubeResetClick OtherActor))
                  (if (Variables|/Game/Hou/BluePrints/BP_CubeResetClick.BP_CubeResetClick_C|GetIsIteam _asbp_cube_reset_click)
                    (bind _aspuzzle_player_controller (Utilities|Casting|CastToPuzzlePlayerController (Class|GameplayStatics|GetPlayerControllerfromID)))
                    (Variables|/Game/PuzzleBP/Blueprints/PuzzlePlayerController.PuzzlePlayerController_C|SetClickCount _aspuzzle_player_controller 0)
                    (Variables|/Game/Hou/BluePrints/BP_CubeResetClick.BP_CubeResetClick_C|SetIsIteam _asbp_cube_reset_click false)
                    (Rendering|SetVisibility (Variables|/Game/Hou/BluePrints/BP_CubeResetClick.BP_CubeResetClick_C|GetSphere _asbp_cube_reset_click) false false)
                    (goto _label_2)
                    (else
                      (goto _label_2))))
                (:4
                  ;[1 1 1] Goal
                  (bind _asbp_cube_goal (Utilities|Casting|CastToBP_CubeGoal OtherActor))
                  (if (Variables|Default|GetIsKey)
                    (Variables|/Game/Hou/BluePrints/BP_CubeGoal.BP_CubeGoal_C|SetSwitchOn _asbp_cube_goal true)
                    (Collision|SetCollisionEnabled (Variables|/Game/Hou/BluePrints/BP_CubeGoal.BP_CubeGoal_C|GetCube1 _asbp_cube_goal) "QueryAndPhysics")
                    (goto _label_3)
                    (else
                      (goto _label))))
                (:5
                  ;[1 1 1] Key
                  (bind _asbp_cube_key (Utilities|Casting|CastToBP_CubeKey OtherActor))
                  (if (Variables|/Game/Hou/BluePrints/BP_CubeKey.BP_CubeKey_C|GetIsIteam _asbp_cube_key)
                    (Variables|Default|SetIsKey true)
                    (Variables|/Game/Hou/BluePrints/BP_CubeKey.BP_CubeKey_C|SetIsIteam _asbp_cube_key false)
                    (Rendering|SetVisibility (Variables|/Game/Hou/BluePrints/BP_CubeKey.BP_CubeKey_C|GetCone _asbp_cube_key) false false)
                    (goto _label_2)
                    (else
                      (goto _label_2))))
                (:6
                  ;[1 1 1] Stair
                  ;;[1 1 1] 上
                  (if (<= (- (.Yaw (Math|Vector|GetYawPitchfromVector (Math|Rotator|GetRotationXVector (Transformation|GetActorRotation)))) (.Yaw (Math|Vector|GetYawPitchfromVector (Math|Rotator|GetRotationXVector (Transformation|GetActorRotation _asbp_cube_base))))) 270.100006)
                    (if (> (- (.Yaw (Math|Vector|GetYawPitchfromVector (Math|Rotator|GetRotationXVector (Transformation|GetActorRotation)))) (.Yaw (Math|Vector|GetYawPitchfromVector (Math|Rotator|GetRotationXVector (Transformation|GetActorRotation _asbp_cube_base))))) 269.899994)
                      _
                      (else
                        (if (<= (- (.Yaw (Math|Vector|GetYawPitchfromVector (Math|Rotator|GetRotationXVector (Transformation|GetActorRotation)))) (.Yaw (Math|Vector|GetYawPitchfromVector (Math|Rotator|GetRotationXVector (Transformation|GetActorRotation _asbp_cube_base))))) -89.900002) :!label _label_5
                          (if (> (- (.Yaw (Math|Vector|GetYawPitchfromVector (Math|Rotator|GetRotationXVector (Transformation|GetActorRotation)))) (.Yaw (Math|Vector|GetYawPitchfromVector (Math|Rotator|GetRotationXVector (Transformation|GetActorRotation _asbp_cube_base))))) -90.099998)
                            _
                            (else
                              (goto _label)))
                          (else
                            (goto _label)))))
                    (else
                      (goto _label_5)))
                  (Variables|Default|SetRotating true)
                  (Variables|Default|SetIsRotateL true :!label _label_6))
                (:7
                  (goto _label_2))
                (:8
                  (goto _label_2)))))
          (elif (Variables|/Game/Hou/BluePrints/BP_CubeBase.BP_CubeBase_C|GetIsActive _asbp_cube_base)
            (switch int (Variables|/Game/Hou/BluePrints/BP_CubeBase.BP_CubeBase_C|GetCubeType _asbp_cube_base)
              (:6
                ;;[1 1 1] 下
                (if (<= (- (.Yaw (Math|Vector|GetYawPitchfromVector (Math|Rotator|GetRotationXVector (Transformation|GetActorRotation)))) (.Yaw (Math|Vector|GetYawPitchfromVector (Math|Rotator|GetRotationXVector (Transformation|GetActorRotation _asbp_cube_base))))) -269.899994)
                  (if (> (- (.Yaw (Math|Vector|GetYawPitchfromVector (Math|Rotator|GetRotationXVector (Transformation|GetActorRotation)))) (.Yaw (Math|Vector|GetYawPitchfromVector (Math|Rotator|GetRotationXVector (Transformation|GetActorRotation _asbp_cube_base))))) -270.100006)
                    _
                    (else
                      (if (<= (- (.Yaw (Math|Vector|GetYawPitchfromVector (Math|Rotator|GetRotationXVector (Transformation|GetActorRotation)))) (.Yaw (Math|Vector|GetYawPitchfromVector (Math|Rotator|GetRotationXVector (Transformation|GetActorRotation _asbp_cube_base))))) 90.099998) :!label _label_7
                        (if (> (- (.Yaw (Math|Vector|GetYawPitchfromVector (Math|Rotator|GetRotationXVector (Transformation|GetActorRotation)))) (.Yaw (Math|Vector|GetYawPitchfromVector (Math|Rotator|GetRotationXVector (Transformation|GetActorRotation _asbp_cube_base))))) 89.900002)
                          _
                          (else
                            (goto _label)))
                        (else
                          (goto _label)))))
                  (else
                    (goto _label_7)))
                (Variables|Default|SetRotating false)
                (goto _label_6)))))))))

(event OnComponentEndOverlap(Box2)
  (params (OverlappedComponent :type Primitive%20Component%20Object%20Reference) (OtherActor :type Actor%20Object%20Reference) (OtherComp :type Primitive%20Component%20Object%20Reference) (OtherBodyIndex :type Integer))
  (bind _playerlayer (Variables|Default|GetPlayerLayer))
  (if (not (Variables|Default|GetIsClockwise))
    (bind _asbp_cube_base (Utilities|Casting|CastToBP_CubeBase OtherActor))
    (if (== (Actor|GetComponentbyClass _asbp_cube_base "/Script/Engine.BoxComponent") OtherComp)
      ;[1 1 1] HeightCube
      (if (== (Variables|/Game/Hou/BluePrints/BP_CubeBase.BP_CubeBase_C|GetCubeLayer _asbp_cube_base) _playerlayer)
        (switch int (Variables|/Game/Hou/BluePrints/BP_CubeBase.BP_CubeBase_C|GetCubeType _asbp_cube_base))
        (elif (> (Variables|/Game/Hou/BluePrints/BP_CubeBase.BP_CubeBase_C|GetCubeLayer _asbp_cube_base) _playerlayer)
          _)))))

(event EventBeginPlay
  (bind _returnvalue (UserInterface|CreateWidget "/Game/Xu/Blueprints/HUD.HUD_C"))
  (UserInterface|Viewport|AddtoViewport _returnvalue 0)
  (Audio|PlaySound2D "/Game/Sound/bgm_chapter1.bgm_chapter1" 1.0 1.0 0.0 0 0))

(event EventTick
  (params (DeltaSeconds :type Float%20%28single-precision%29))
  (if (Variables|Default|GetRotate360)
    ;[1 1 1] 360
    (Transformation|AddActorLocalRotation "0,180.000000, 0" false false)
    (Variables|Default|SetRotate360 false)
    (Pawn|Input|AddMovementInput (Transformation|GetActorForwardVector) 1.0 false :!label _label)
    (else
      ;[1 1 1] 左转
      (if (Variables|Default|GetIsRotateL)
        (if (Variables|Default|GetIsRightAngle)
          (if (Variables|Default|GetIsClockwise)
            (Transformation|AddActorLocalRotation "0,90.000000, 0" false false)
            (else
              (Transformation|AddActorLocalRotation "0,-90.000000, 0" false false)))
          (Variables|Default|SetIsRotateL false)
          (else
            (if (Variables|Default|GetIsClockwise)
              (Transformation|AddActorLocalRotation "0,-90.000000, 0" false false)
              (else
                (Transformation|AddActorLocalRotation "0,90.000000, 0" false false)))
            (Variables|Default|SetIsRotateL false)))
        (else
          ;[1 1 1] 前方，右转
          (if (Variables|Default|GetIsRotateF)
            (if (Variables|Default|GetIsClockwise)
              (Transformation|AddActorLocalRotation "0,90.000000, 0" false false)
              (else
                (Transformation|AddActorLocalRotation "0,-90.000000, 0" false false)))
            (Variables|Default|SetIsRotateF false)
            (Variables|Default|SetRotating false)
            (Variables|Default|SetIsRightAngle false)
            (else
              (goto _label))))))))

(fn ConstructionScript)