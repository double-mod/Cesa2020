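; BP_TestBox is a pushable box that BP_AutoCharacter_2 can shove across cubes, sliding along a stored direction each tick while IsMove is set.
; BoxTestA takes that direction from the character's contact and enables the ForwardBox probe, and also marks overlapped cubes as occupied on top.
; ForwardBox checks the next cube, either snapping and stopping the box or enabling BoxTestB, which flags the character ready to push or rotate-push.
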(event OnComponentBeginOverlap(ForwardBox)
  (params (OverlappedComponent :type Primitive%20Component%20Object%20Reference) (OtherActor :type Actor%20Object%20Reference) (OtherComp :type Primitive%20Component%20Object%20Reference) (OtherBodyIndex :type Integer) (bFromSweep :type Boolean) (SweepResult :type Hit%20Result%20Structure%20%28by%20ref%29))
  (bind _asbp_cube_base (Utilities|Casting|CastToBP_CubeBase OtherActor))
  (if (== OtherComp (Variables|/Game/Hou/BluePrints/BP_CubeBase.BP_CubeBase_C|GetBox _asbp_cube_base))
    (switch int (Variables|/Game/Hou/BluePrints/BP_CubeBase.BP_CubeBase_C|GetCubeType _asbp_cube_base)
      (:0
        (if (Variables|/Game/Hou/BluePrints/BP_CubeBase.BP_CubeBase_C|GetIsActive _asbp_cube_base) :!label _label
          (if (Variables|/Game/Hou/BluePrints/BP_CubeBase.BP_CubeBase_C|GetTopIsTestBox _asbp_cube_base)
            (Variables|Default|SetForwardTest false :!label _label_2)
            (Variables|Default|SetIsMove false)
            (Collision|SetCollisionEnabled (Variables|Default|GetForwardBox) "NoCollision")
            (Transformation|SetActorLocation (- (Math|Vector|MakeVector (.X (Math|Vector|BreakVector (Transformation|GetActorLocation _asbp_cube_base))) (.Y (Math|Vector|BreakVector (Transformation|GetActorLocation _asbp_cube_base))) (.Z (Math|Vector|BreakVector (Transformation|GetActorLocation)))) (* (Variables|Default|GetDiretion) (Math|Vector|MakeVector 1e+02 1e+02 0.0))) false false)
            (else
              (Variables|Default|SetForwardTest true)
              (if (not (Variables|Default|GetIsMove))
                (Collision|SetCollisionEnabled (Variables|Default|GetBoxTestB) "QueryOnly"))))
          (else
            (goto _label_2))))
      (:3
        (bind _asbp_cube_memory (Utilities|Casting|CastToBP_CubeMemory _asbp_cube_base))
        (if (Variables|/Game/Hou/BluePrints/Test/BP_CubeMemory.BP_CubeMemory_C|GetIsInstantiation _asbp_cube_memory)
          (goto _label_2)
          (else
            (goto _label)))))))

(event OnComponentBeginOverlap(BoxTestA)
  (params (OverlappedComponent :type Primitive%20Component%20Object%20Reference) (OtherActor :type Actor%20Object%20Reference) (OtherComp :type Primitive%20Component%20Object%20Reference) (OtherBodyIndex :type Integer) (bFromSweep :type Boolean) (SweepResult :type Hit%20Result%20Structure%20%28by%20ref%29))
  (bind _asbp_auto_character_2 (Utilities|Casting|CastToBP_AutoCharacter_2 OtherActor)
    (:then
      (if (== (Variables|/Game/Hou/BluePrints/Test/BP_AutoCharacter_2.BP_AutoCharacter_2_C|GetBoxBegin _asbp_auto_character_2) OtherComp)
        (if (not (Variables|Default|GetSideCollision))
          (Variables|Default|SetDiretion (Math|Vector|Normalize (Transformation|GetActorForwardVector _asbp_auto_character_2)))
          (Transformation|SetWorldRotation (Variables|Default|GetChildActor) (Transformation|GetActorRotation _asbp_auto_character_2) false false)
          (Collision|SetCollisionEnabled (Variables|Default|GetForwardBox) "QueryOnly"))
        (elif (Variables|/Game/Hou/BluePrints/Test/BP_AutoCharacter_2.BP_AutoCharacter_2_C|GetIsClockwise _asbp_auto_character_2)
          (if (== OtherComp (Variables|/Game/Hou/BluePrints/Test/BP_AutoCharacter_2.BP_AutoCharacter_2_C|GetBox1 _asbp_auto_character_2))
            (Variables|Default|SetDiretion (Math|Vector|Normalize (* (Transformation|GetActorRightVector _asbp_auto_character_2) -1)))
            (Transformation|SetWorldRotation (Variables|Default|GetChildActor) (Math|Rotator|MakeRotator 0.0 0.0 (+ (.Yaw (Math|Rotator|BreakRotator (Transformation|GetActorRotation _asbp_auto_character_2))) -9e+01)) false false)
            (Collision|SetCollisionEnabled (Variables|Default|GetForwardBox) "QueryOnly")
            (Variables|Default|SetSideCollision true)))))
    (:CastFailed
      (bind _asbp_cube_base (Utilities|Casting|CastToBP_CubeBase OtherActor))
      (if (== OtherComp (Variables|/Game/Hou/BluePrints/BP_CubeBase.BP_CubeBase_C|GetBox _asbp_cube_base))
        (switch int (Variables|/Game/Hou/BluePrints/BP_CubeBase.BP_CubeBase_C|GetCubeType _asbp_cube_base)
          (:0
            _)
          (:1
            _)
          (:3
            _))
        (Variables|/Game/Hou/BluePrints/BP_CubeBase.BP_CubeBase_C|SetTopIsTestBox _asbp_cube_base true)))))

(event OnComponentBeginOverlap(BoxTestB)
  (params (OverlappedComponent :type Primitive%20Component%20Object%20Reference) (OtherActor :type Actor%20Object%20Reference) (OtherComp :type Primitive%20Component%20Object%20Reference) (OtherBodyIndex :type Integer) (bFromSweep :type Boolean) (SweepResult :type Hit%20Result%20Structure%20%28by%20ref%29))
  (bind _asbp_auto_character_2 (Utilities|Casting|CastToBP_AutoCharacter_2 OtherActor))
  (if (== (Variables|/Game/Hou/BluePrints/Test/BP_AutoCharacter_2.BP_AutoCharacter_2_C|GetBoxBegin _asbp_auto_character_2) OtherComp)
    (Variables|/Game/Hou/BluePrints/Test/BP_AutoCharacter_2.BP_AutoCharacter_2_C|SetPushReady _asbp_auto_character_2 true)
    (Collision|SetCollisionEnabled (Variables|Default|GetBoxTestB) "NoCollision" :!label _label)
    (elif (Variables|/Game/Hou/BluePrints/Test/BP_AutoCharacter_2.BP_AutoCharacter_2_C|GetIsClockwise _asbp_auto_character_2)
      (if (== OtherComp (Variables|/Game/Hou/BluePrints/Test/BP_AutoCharacter_2.BP_AutoCharacter_2_C|GetBox1 _asbp_auto_character_2))
        (Variables|/Game/Hou/BluePrints/Test/BP_AutoCharacter_2.BP_AutoCharacter_2_C|SetPushRotateReady _asbp_auto_character_2 true)
        (goto _label)))))

(event Custom|CubeMove
  (bind _defaultsceneroot (Variables|Default|GetDefaultSceneRoot))
  (bind _returnvalue (Transformation|GetWorldTransform _defaultsceneroot))
  (bind (_location _rotation _scale) (Math|Transform|BreakTransform _returnvalue))
  (Transformation|SetActorTransform (Math|Transform|MakeTransform (+ (* (Math|Vector|Normalize (Variables|Default|GetDiretion) 0.001) (* (Utilities|Time|GetWorldDeltaSeconds) (Variables|Default|GetSpeed))) _location) _rotation _scale)))

(event EventBeginPlay)

(event Collision|EventActorBeginOverlap
  (params (OtherActor :type Actor%20Object%20Reference)))

(event EventTick
  (params (DeltaSeconds :type Float%20%28single-precision%29))
  (if (Variables|Default|GetIsMove)
    (CallFunction|CubeMove)))

(fn ConstructionScript)