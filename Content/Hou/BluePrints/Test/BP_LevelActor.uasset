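; Level actor that detects puzzle completion when MemoryCount reaches zero and runs the clear sequence.
; BeginPlay passes WinType to PuzzlePlayerController, and TestWin reports completion and arms AnimStart.
; Tick stops AutoCharacter, then once armed shows the GameClear widget, swaps BGM for success audio and animates every Memory.
; WinType 0 chains timelines driving wave and blur material parameter collections, then resets the wave and sets the controller's WinFlag.
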(event EventBeginPlay
  (bind _aspuzzle_player_controller (Utilities|Casting|CastToPuzzlePlayerController (Class|GameplayStatics|GetPlayerControllerfromID)))
  (Variables|/Game/PuzzleBP/Blueprints/PuzzlePlayerController.PuzzlePlayerController_C|SetWinType _aspuzzle_player_controller (Variables|Default|GetWinType)))

(event Collision|EventActorBeginOverlap
  (params (OtherActor :type Actor%20Object%20Reference)))

(event EventTick
  (params (DeltaSeconds :type Float%20%28single-precision%29))
  (if (== (Variables|Default|GetMemoryCount) 0)
    (Variables|/Game/Hou/BluePrints/Test/BP_AutoCharacter_2.BP_AutoCharacter_2_C|SetWinStop (Variables|Default|GetAutoCharacter) true)
    (if (Variables|Default|GetAnimStart)
      (bind _returnvalue (UserInterface|CreateWidget "/Game/Xu/Blueprints/GameClear.GameClear_C"))
      (UserInterface|Viewport|AddtoViewport _returnvalue 0)
      (Variables|Default|SetAnimStart false)
      (Audio|PlaySound2D "/Game/Sound/se_success2.se_success2" 1.0 1.0 0.0 0 0)
      (Default|StopBGM (Variables|Default|GetAutoCharacter))
      (for _array_element (Variables|Default|GetMemory)
        (Default|PlayAnim _array_element))
      (switch int (Variables|Default|GetWinType)
        (:0
          (Timeline|WaitAnim Play
            (:Update
              (Rendering|Material|SetScalarParameterValue "/Game/Hou/Materials/Wave/MPC_wave.MPC_wave" "Speed" -1.0 :!class /Script/Engine.KismetMaterialLibrary)
              (Rendering|Material|SetScalarParameterValue "/Game/Hou/Materials/Wave/MPC_wave.MPC_wave" "Size" 5.0 :!class /Script/Engine.KismetMaterialLibrary))
            (:Finished
              (bind _blur (Timeline|Blur Play)
                (:Update
                  (Rendering|Material|SetScalarParameterValue "/Game/Hou/Materials/Blur/MPC_Blur.MPC_Blur" "BlurPower" _blur :!class /Script/Engine.KismetMaterialLibrary))
                (:Finished
                  (Rendering|Material|SetScalarParameterValue "/Game/Hou/Materials/Wave/MPC_wave.MPC_wave" "Speed" 0.0 :!class /Script/Engine.KismetMaterialLibrary)
                  (Rendering|Material|SetScalarParameterValue "/Game/Hou/Materials/Wave/MPC_wave.MPC_wave" "Size" 1.0 :!class /Script/Engine.KismetMaterialLibrary)
                  (bind _aspuzzle_player_controller (Utilities|Casting|CastToPuzzlePlayerController (Class|GameplayStatics|GetPlayerControllerfromID)))
                  (Variables|/Game/PuzzleBP/Blueprints/PuzzlePlayerController.PuzzlePlayerController_C|SetWinFlag _aspuzzle_player_controller true))))))))))

(fn ConstructionScript)

(fn TestWin
  (if (== (Variables|Default|GetMemoryCount) 0)
    (Variables|Default|SetAnimStart true)
    (return true)
    (else
      (return false))))