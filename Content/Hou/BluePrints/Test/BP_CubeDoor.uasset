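; BP_CubeDoor is a door that redirects a moving BP_TestBox cube, apparently for 90-degree turns.
; Box overlaps with the cube's BoxTestA track the cube and its incoming direction.
; Once it halts, Tick uses ChangeAngle's two-entry direction lookup to re-orient it and enable its forward probe.
; A later Tick relaunches the cube with a turn sound if it reports BoxReady, otherwise latches StopDoorEvent.
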(event OnComponentBeginOverlap(Box)
  (params (OverlappedComponent :type Primitive%20Component%20Object%20Reference) (OtherActor :type Actor%20Object%20Reference) (OtherComp :type Primitive%20Component%20Object%20Reference) (OtherBodyIndex :type Integer) (bFromSweep :type Boolean) (SweepResult :type Hit%20Result%20Structure%20%28by%20ref%29))
  (bind _asbp_test_box (Utilities|Casting|CastToBP_TestBox OtherActor))
  (if (== OtherComp (Variables|/Game/Hou/BluePrints/Test/BP_TestBox.BP_TestBox_C|GetBoxTestA _asbp_test_box))
    (Variables|Default|SetTestBox _asbp_test_box)
    (Variables|Default|SetTestBoxDirection (Variables|/Game/Hou/BluePrints/Test/BP_TestBox.BP_TestBox_C|GetDiretion _asbp_test_box))))

(event OnComponentEndOverlap(Box)
  (params (OverlappedComponent :type Primitive%20Component%20Object%20Reference) (OtherActor :type Actor%20Object%20Reference) (OtherComp :type Primitive%20Component%20Object%20Reference) (OtherBodyIndex :type Integer))
  (bind _asbp_test_box (Utilities|Casting|CastToBP_TestBox OtherActor))
  (if (== OtherComp (Variables|/Game/Hou/BluePrints/Test/BP_TestBox.BP_TestBox_C|GetBoxTestA _asbp_test_box))
    (if (== _asbp_test_box (Variables|Default|GetTestBox))
      (Variables|Default|SetTopIsTestBox false)
      (Variables|/Game/Hou/BluePrints/Test/BP_TestBox.BP_TestBox_C|SetPassDoor (Variables|Default|GetTestBox) false)
      (Variables|Default|SetTestBox 0)
      (Variables|Default|SetReady false))))

(event EventBeginPlay
  (|CallParentFunction) ; 此节点被禁用，将不会被调用。\n从引脚连出引线来编译功能。
)

(event Collision|EventActorBeginOverlap
  (params (OtherActor :type Actor%20Object%20Reference)))

(event EventTick
  (params (DeltaSeconds :type Float%20%28single-precision%29))
  (bind _testbox (Variables|Default|GetTestBox))
  (|CallParentFunction DeltaSeconds)
  (if (!= _testbox 0)
    (if (not (Variables|/Game/Hou/BluePrints/Test/BP_TestBox.BP_TestBox_C|GetIsMove _testbox))
      (if (Variables|Default|GetReady)
        (if (not (Variables|Default|GetStopDoorEvent))
          (if (Variables|/Game/Hou/BluePrints/Test/BP_TestBox.BP_TestBox_C|GetBoxReady _testbox)
            (Collision|SetCollisionEnabled (Variables|/Game/Hou/BluePrints/Test/BP_TestBox.BP_TestBox_C|GetBoxTestB _testbox) "NoCollision")
            (Default|MoveStart _testbox)
            (Default|Stop _testbox)
            (Variables|Default|SetReady false)
            (Variables|/Game/Hou/BluePrints/Test/BP_TestBox.BP_TestBox_C|SetBoxReady _testbox false)
            (Variables|/Game/Hou/BluePrints/Test/BP_TestBox.BP_TestBox_C|SetDoorReady _testbox false)
            (Audio|PlaySound2D "/Game/Sound/se_90turn.se_90turn" 1.0 1.0 0.0 0 0)
            (else
              (Variables|Default|SetStopDoorEvent true))))
        (else
          (Variables|Default|SetReady true)
          (Variables|Default|SetStopDoorEvent false)
          (bind (_output _rotation) (CallFunction|ChangeAngle))
          (Variables|/Game/Hou/BluePrints/Test/BP_TestBox.BP_TestBox_C|SetDiretion _testbox _output)
          (Transformation|SetWorldRotation (Variables|/Game/Hou/BluePrints/Test/BP_TestBox.BP_TestBox_C|GetChildActor _testbox) _rotation false false)
          (Variables|/Game/Hou/BluePrints/Test/BP_TestBox.BP_TestBox_C|SetNumTwoTest _testbox false)
          (Variables|/Game/Hou/BluePrints/Test/BP_TestBox.BP_TestBox_C|SetHeadBox _testbox false)
          (Variables|/Game/Hou/BluePrints/Test/BP_TestBox.BP_TestBox_C|SetBackTestBox _testbox 0)
          (Variables|/Game/Hou/BluePrints/Test/BP_TestBox.BP_TestBox_C|SetDoorReady _testbox true)
          (Collision|SetCollisionEnabled (Variables|/Game/Hou/BluePrints/Test/BP_TestBox.BP_TestBox_C|GetForwardBox _testbox) "QueryOnly"))))))

(fn ConstructionScript
  (|CallParentFunction))

(fn ChangeAngle
  (if (Math|Vector|Equal(Vector) (Utilities|Array|Get(acopy) (Variables|Default|GetInputDir)) (Variables|Default|GetTestBoxDirection) 0.0001)
    (return (Utilities|Array|Get(acopy) (Variables|Default|GetOutputDir)) (Utilities|Array|Get(acopy) (Variables|Default|GetOutputRotation)))
    (elif (Math|Vector|Equal(Vector) (Utilities|Array|Get(acopy) (Variables|Default|GetInputDir) 1) (Variables|Default|GetTestBoxDirection) 0.0001)
      (return (Utilities|Array|Get(acopy) (Variables|Default|GetOutputDir) 1) (Utilities|Array|Get(acopy) (Variables|Default|GetOutputRotation) 1))
      (else
        (Development|PrintString "door bug")))))