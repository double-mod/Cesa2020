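; BP_CubeMemory is a test actor that remembers a BP_TestBox overlapping its Box component.
; On begin overlap, it stores that actor in TestBox if the touching component is the actor's BoxTestA.
; When BoxTestA leaves, it clears TestBox and sets TopIsTestBox to false, a flag this graph never sets true.
; Tick only calls its parent, and the construction script adds no logic.
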(event OnComponentBeginOverlap(Box)
  (params (OverlappedComponent :type Primitive%20Component%20Object%20Reference) (OtherActor :type Actor%20Object%20Reference) (OtherComp :type Primitive%20Component%20Object%20Reference) (OtherBodyIndex :type Integer) (bFromSweep :type Boolean) (SweepResult :type Hit%20Result%20Structure%20%28by%20ref%29))
  (bind _asbp_test_box (Utilities|Casting|CastToBP_TestBox OtherActor))
  (if (== (Variables|/Game/Hou/BluePrints/Test/BP_TestBox.BP_TestBox_C|GetBoxTestA _asbp_test_box) OtherComp)
    (Variables|Default|SetTestBox _asbp_test_box)))

(event OnComponentEndOverlap(Box)
  (params (OverlappedComponent :type Primitive%20Component%20Object%20Reference) (OtherActor :type Actor%20Object%20Reference) (OtherComp :type Primitive%20Component%20Object%20Reference) (OtherBodyIndex :type Integer))
  (bind _asbp_test_box (Utilities|Casting|CastToBP_TestBox OtherActor))
  (if (== (Variables|/Game/Hou/BluePrints/Test/BP_TestBox.BP_TestBox_C|GetBoxTestA _asbp_test_box) OtherComp)
    (Variables|Default|SetTopIsTestBox false)
    (Variables|Default|SetTestBox 0)))

(event EventBeginPlay
  (|CallParentFunction) ; This node is disabled and will not be called.\nDrag off pins to build functionality.
)

(event Collision|EventActorBeginOverlap
  (params (OtherActor :type Actor%20Object%20Reference)))

(event EventTick
  (params (DeltaSeconds :type Float%20%28single-precision%29))
  (|CallParentFunction DeltaSeconds))

(fn ConstructionScript
  (|CallParentFunction))