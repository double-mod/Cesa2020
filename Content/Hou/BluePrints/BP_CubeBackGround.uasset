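; BP_CubeBackGround is an actor with a Cube component that, judging by its name, serves as background scenery.
; On BeginPlay it runs the parent logic, then makes the cube visible and disables its collision, so it is purely visual.
; Construction and the delta-time event only forward to the parent class, and a duplicate of the visibility and collision setup is left unconnected.
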(event Custom|CustomEvent
  (params (DeltaSeconds :type Float%20%28single-precision%29))
  (|CallParentFunction DeltaSeconds))

(event EventBeginPlay
  (bind _cube (Variables|Default|GetCube))
  (|CallParentFunction)
  (Rendering|SetVisibility _cube true false)
  (Collision|SetCollisionEnabled _cube "NoCollision"))

(event Collision|EventActorBeginOverlap
  (params (OtherActor :type Actor%20Object%20Reference)))

(fn ConstructionScript
  (|CallParentFunction))