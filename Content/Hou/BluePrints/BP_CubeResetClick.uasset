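; Puzzle click-reset pickup that spins its child actor while active and clears the player's click count when switched off.
; BeginPlay hides the Cube mesh and disables its collision.
; While active, Tick rotates the child actor and sets Ready to match whether DownCube is active.
; OffIteam hides Cube1, disables its and Box's collision, deactivates the actor and zeroes ClickCount on the PuzzlePlayerController.
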(event Custom|OffIteam
  (bind _cube1 (Variables|Default|GetCube1))
  (Rendering|SetVisibility _cube1 false false)
  (Collision|SetCollisionEnabled (Variables|Default|GetBox) "NoCollision")
  (Collision|SetCollisionEnabled _cube1 "NoCollision")
  (Variables|Default|SetIsActive false)
  (bind _aspuzzle_player_controller (Utilities|Casting|CastToPuzzlePlayerController (Class|GameplayStatics|GetPlayerControllerfromID)))
  (Variables|/Game/PuzzleBP/Blueprints/PuzzlePlayerController.PuzzlePlayerController_C|SetClickCount _aspuzzle_player_controller 0))

(event EventBeginPlay
  (bind _cube (Variables|Default|GetCube))
  (|CallParentFunction)
  (Collision|SetCollisionEnabled _cube "NoCollision")
  (Rendering|SetVisibility _cube false false))

(event Collision|EventActorBeginOverlap
  (params (OtherActor :type Actor%20Object%20Reference)))

(event EventTick
  (params (DeltaSeconds :type Float%20%28single-precision%29))
  (|CallParentFunction DeltaSeconds)
  (if (Variables|Default|GetIsActive)
    (Transformation|AddLocalRotation (Variables|Default|GetChildActor) "0,2.000000, 0" false false)
    (if (Variables|/Game/Hou/BluePrints/BP_CubeBase.BP_CubeBase_C|GetIsActive (Variables|Default|GetDownCube))
      (Variables|Default|SetReady true)
      (else
        (Variables|Default|SetReady false)))))

(fn ConstructionScript
  (|CallParentFunction))