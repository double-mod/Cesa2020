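; BP_CubeTimer is a countdown cube that changes material as DisappearCount drops, then dissolves away at zero.
; Tick polls the count, which is changed outside this graph, to pick from the Mat array.
; At zero it disables collision and activity, and updates its state and DownCube's if one sits below.
; A timeline then drives the "Amount" material parameter and calls HideCube, with a dynamic material created every dissolving tick.
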(event EventBeginPlay
  (|CallParentFunction))

(event Collision|EventActorBeginOverlap
  (params (OtherActor :type Actor%20Object%20Reference)))

(event EventTick
  (params (DeltaSeconds :type Float%20%28single-precision%29))
  (bind _disappearcount (Variables|Default|GetDisappearCount))
  (bind _mat (Variables|Default|Getmat))
  (bind _cube (Variables|Default|GetCube))
  (|CallParentFunction DeltaSeconds)
  (if (Variables|Default|GetIsDissolve)
    (Rendering|Material|CreateDynamicMaterialInstance _cube 0 (Rendering|Material|GetMaterial _cube 0) "None" :!class /Script/Engine.PrimitiveComponent)
    (bind _newtrack_0 (Timeline|Timeline_0 Play)
      (:Update
        (Rendering|Material|SetScalarParameterValueonMaterials (Variables|Default|GetCube) "Amount" _newtrack_0))
      (:Finished
        (CallFunction|HideCube)))
    (elif (== _disappearcount 2)
      (Rendering|Material|SetMaterial _cube 0 (Utilities|Array|Get(acopy) _mat 2))
      (elif (== _disappearcount 1)
        (Rendering|Material|SetMaterial _cube 0 (Utilities|Array|Get(acopy) _mat 1))
        (elif (== _disappearcount 0)
          (Rendering|Material|SetMaterial _cube 0 (Utilities|Array|Get(acopy) _mat))
          (Variables|Default|SetIsDissolve true)
          (Variables|Default|SetIsActive false)
          (Collision|SetCollisionEnabled (Variables|Default|GetCube) "NoCollision")
          (if (Variables|Default|GetHaveDown)
            (Variables|/Game/Hou/BluePrints/BP_CubeBase.BP_CubeBase_C|SetHaveTop (Variables|Default|GetDownCube) false)
            (Variables|Default|SetCubeType 0)))))))

(fn ConstructionScript
  (|CallParentFunction))