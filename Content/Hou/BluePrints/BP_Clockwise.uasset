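; BP_Clockwise is a clickable puzzle cube that can be deleted by dissolving it.
; A click on an eligible cube disables collision and starts dissolving, within a three-click limit on PuzzlePlayerController.
; If stacked on another, it also clears that cube's HaveTop, increments the click count and plays a sound.
; Tick drives a brief custom-depth outline for uncovered cubes and the material-parameter dissolve timeline, which ends in HideCube.
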(event OnClicked(Cube)
  (params (TouchedComponent :type Primitive%20Component%20Object%20Reference) (ButtonPressed :type Key%20Structure :default "None"))
  (if (not (Variables|Default|GetIsDissolve))
    (if (Variables|Default|GetIsDisappear)
      (bind _aspuzzle_player_controller (Utilities|Casting|CastToPuzzlePlayerController (Class|GameplayStatics|GetPlayerControllerfromID)))
      (if (< (Variables|/Game/PuzzleBP/Blueprints/PuzzlePlayerController.PuzzlePlayerController_C|GetClickCount _aspuzzle_player_controller) 3)
        (if (not (Variables|Default|GetIsPlayer))
          (if (Variables|Default|GetIsActive)
            (Variables|Default|SetIsDissolve true)
            (Variables|Default|SetIsActive false)
            (Collision|SetCollisionEnabled (Variables|Default|GetCube) "NoCollision")
            (if (Variables|Default|GetHaveDown)
              (Variables|/Game/Hou/BluePrints/BP_CubeBase.BP_CubeBase_C|SetHaveTop (Variables|Default|GetDownCube) false)
              (bind _result (Math|Integer|IncrementInt (Variables|/Game/PuzzleBP/Blueprints/PuzzlePlayerController.PuzzlePlayerController_C|GetClickCount _aspuzzle_player_controller))
                (:%20%20
                  (Variables|/Game/PuzzleBP/Blueprints/PuzzlePlayerController.PuzzlePlayerController_C|SetClickCount _aspuzzle_player_controller _result)
                  (Audio|PlaySoundatLocation "/Game/Sound/memory_delete1.memory_delete1" (Transformation|GetActorLocation) "0, 0, 0" 1.0 1.0 0.0 0 0 0)
                  (Variables|Default|SetCubeType 0))))))))))

(event Custom|OpenOutline
  (if (not (Variables|Default|GetHaveTop))
    (Utilities|Time|SetTimerbyEvent (delegate Custom|CloseOutline) 0.5)
    (Rendering|SetRenderCustomDepth (Variables|Default|GetCube) true)
    (Variables|Default|SetIsOutline false)))

(event Custom|CloseOutline
  (Rendering|SetRenderCustomDepth (Variables|Default|GetCube) false)
  (Variables|Default|SetIsOutline false))

(event EventBeginPlay
  (|CallParentFunction))

(event Collision|EventActorBeginOverlap
  (params (OtherActor :type Actor%20Object%20Reference)))

(event EventTick
  (params (DeltaSeconds :type Float%20%28single-precision%29))
  (bind _cube (Variables|Default|GetCube))
  (|CallParentFunction DeltaSeconds)
  (if (Variables|Default|GetIsDisappear)
    (if (Variables|Default|GetIsOutline)
      (CallFunction|OpenOutline))
    (if (Variables|Default|GetIsDissolve)
      (Rendering|Material|CreateDynamicMaterialInstance _cube 0 (Rendering|Material|GetMaterial _cube 0) "None" :!class /Script/Engine.PrimitiveComponent)
      (bind _newtrack_0 (Timeline|Timeline_0 Play)
        (:Update
          (Rendering|Material|SetScalarParameterValueonMaterials (Variables|Default|GetCube) "Amount" _newtrack_0))
        (:Finished
          (CallFunction|HideCube))))))

(fn ConstructionScript
  (|CallParentFunction))