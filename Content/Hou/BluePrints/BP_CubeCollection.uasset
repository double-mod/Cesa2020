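; BP_CubeCollection is a collectible puzzle cube that spins while active and adds to the player's collection count.
; Tick rotates the cube and sets Ready to mirror whether the linked DownCube is active.
; OffIteam hides the cube, disables cube and box collision, clears IsActive and increments CollectionCount on PuzzlePlayerController.
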(event Custom|OffIteam
  (bind _cube (Variables|Default|GetCube))
  (Rendering|SetVisibility _cube false false)
  (Collision|SetCollisionEnabled (Variables|Default|GetBox) "NoCollision")
  (Collision|SetCollisionEnabled _cube "NoCollision")
  (Variables|Default|SetIsActive false)
  (bind _aspuzzle_player_controller (Utilities|Casting|CastToPuzzlePlayerController (Class|GameplayStatics|GetPlayerControllerfromID)))
  (bind _result (Math|Integer|IncrementInt (Variables|/Game/PuzzleBP/Blueprints/PuzzlePlayerController.PuzzlePlayerController_C|GetCollectionCount _aspuzzle_player_controller))
    (:%20%20
      (Variables|/Game/PuzzleBP/Blueprints/PuzzlePlayerController.PuzzlePlayerController_C|SetCollectionCount _aspuzzle_player_controller _result))))

(event EventBeginPlay
  (|CallParentFunction)
  (Collision|SetCollisionEnabled (Variables|Default|GetCube) "NoCollision"))

(event Collision|EventActorBeginOverlap
  (params (OtherActor :type Actor%20Object%20Reference)))

(event EventTick
  (params (DeltaSeconds :type Float%20%28single-precision%29))
  (|CallParentFunction DeltaSeconds)
  (if (Variables|Default|GetIsActive)
    (Transformation|AddLocalRotation (Variables|Default|GetCube) "0,2.000000, 0" false false)
    (if (Variables|/Game/Hou/BluePrints/BP_CubeBase.BP_CubeBase_C|GetIsActive (Variables|Default|GetDownCube))
      (Variables|Default|SetReady true)
      (else
        (Variables|Default|SetReady false)))))

(fn ConstructionScript
  (|CallParentFunction))