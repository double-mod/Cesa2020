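; BP_CubeBase is a cube Blueprint, apparently a base class, whose starting visibility and collision depend on two flags.
; On BeginPlay the cube is hidden with no collision only when IsDisappear is set and IsActive is not; otherwise it is visible with query and physics collision.
; HideCube turns off visibility but leaves collision untouched, and TestLOG prints the cube component's path name for debugging.
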(event Custom|HideCube
  (Rendering|SetVisibility (Variables|Default|GetCube) false false))

(event Custom|TestLOG
  (Development|PrintString (Class|KismetSystemLibrary|GetPathName (Variables|Default|GetCube))))

(event EventBeginPlay
  (bind _cube (Variables|Default|GetCube))
  (bind _cube_2 (Variables|Default|GetCube))
  (if (Variables|Default|GetIsDisappear)
    (if (Variables|Default|GetIsActive)
      (Rendering|SetVisibility _cube true false :!label _label)
      (Collision|SetCollisionEnabled _cube "QueryAndPhysics")
      (else
        (Rendering|SetVisibility _cube_2 false false)
        (Collision|SetCollisionEnabled _cube_2 "NoCollision")))
    (else
      (goto _label))))

(event EventTick
  (params (DeltaSeconds :type Float%20%28single-precision%29)))

(fn ConstructionScript)