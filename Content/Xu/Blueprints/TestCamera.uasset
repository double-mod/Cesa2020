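; Test camera pawn that rotates in yaw steps and hops between points in a spawn list.
; Right mouse advances the target yaw in fixed increments, and mouse wheel up cycles to the next spawn point's transform.
; Every tick eases the player controller's control rotation and the spring arm's world location toward those targets using RInterpTo and VInterpTo; only the target's location is applied.
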(event Custom|Turn
  (bind _returnvalue (Pawn|GetControlRotation :!class /Script/Engine.Pawn))
  (bind _rotateangle (Variables|Default|GetrotateAngle))
  (if (Utilities|Enum|NotEqual(Enum) _returnvalue _rotateangle)
    (Pawn|SetControlRotation (Game|GetPlayerController 0) (Math|Interpolation|RInterpTo _returnvalue _rotateangle (Utilities|Time|GetWorldDeltaSeconds) 5.0))))

(event Custom|TransformCamera
  (bind _springarm (Variables|Default|GetSpringArm))
  (bind _tranformto (Variables|Default|GetTranformTo))
  (bind _returnvalue (Transformation|GetWorldTransform _springarm))
  (if (Math|Vector|NotEqual(Vector) (.location _tranformto) (.location _returnvalue) 0.0001)
    (Transformation|SetWorldLocation (Variables|Default|GetSpringArm) (Math|Interpolation|VInterpTo (.location _returnvalue) (.location _tranformto) (Utilities|Time|GetWorldDeltaSeconds) 5.0) false false)))

(event EventBeginPlay)

(event Collision|EventActorBeginOverlap
  (params (OtherActor :type Actor%20Object%20Reference)))

(event EventTick
  (params (DeltaSeconds :type Float%20%28single-precision%29))
  (CallFunction|Turn)
  (CallFunction|TransformCamera))

(event Input|MouseEvents|RightMouseButton
  (params (Key :type Key%20Structure :default "None"))
  (:Pressed
    (if (< (.yaw (Variables|Default|GetrotateAngle)) 3.6e+02)
      (Variables|Default|SetrotateAngle (Math|Rotator|MakeRotator 0.0 0.0 (+ (.yaw (Variables|Default|GetrotateAngle)) 3e+01)))
      (else
        (Variables|Default|SetrotateAngle (Math|Rotator|MakeRotator 0.0 0.0 0.0))))))

(event Input|MouseEvents|MouseWheelUp
  (params (Key :type Key%20Structure :default "None"))
  (bind _spawnlist (Variables|Default|GetSpawnList))
  (:Pressed
    (if (< (Variables|Default|GetnextSpawnPoint) (Utilities|Array|LastIndex _spawnlist))
      (Variables|Default|SetnextSpawnPoint (+ (Variables|Default|GetnextSpawnPoint) 1))
      (else
        (Variables|Default|SetnextSpawnPoint 0)))
    (Variables|Default|SetTranformTo (Transformation|GetWorldTransform (Variables|/Script/Engine.Actor|GetRootComponent (Utilities|Array|Get(acopy) _spawnlist (Variables|Default|GetnextSpawnPoint)))))))

(fn ConstructionScript)