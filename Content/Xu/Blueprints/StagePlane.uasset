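; StagePlane is an actor whose plane displays a capture image for the current stage or chapter through the OldMovieEffect material.
; On BeginPlay it applies a dynamic instance of that material to the plane.
; Every Tick it sets StageTexture from the GlobalValue game instance's StageMap result capture when InNewStage is true.
; Otherwise it uses the current chapter's default capture from PuzzlePlayerController's ChapterMap.
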(event EventBeginPlay
  (bind _plane (Variables|Default|GetPlane))
  (bind _returnvalue (Rendering|Material|CreateDynamicMaterialInstance _plane 0 "/Game/Xu/Material/OldMovieEffect.OldMovieEffect" "None" :!class /Script/Engine.PrimitiveComponent))
  (Rendering|Material|SetMaterial _plane 0 _returnvalue))

(event EventTick
  (params (DeltaSeconds :type Float%20%28single-precision%29))
  (bind _asglobal_value (Utilities|Casting|CastToGlobalValue (Game|GetGameInstance)))
  (if (Variables|/Game/Xu/Blueprints/GlobalValue.GlobalValue_C|GetInNewStage _asglobal_value)
    (Rendering|Material|SetTextureParameterValue (stale EventBeginPlay _returnvalue) "StageTexture" (.resultcapture (.Value (Utilities|Map|Find (Variables|/Game/Xu/Blueprints/GlobalValue.GlobalValue_C|GetStageMap _asglobal_value) (Variables|/Game/Xu/Blueprints/GlobalValue.GlobalValue_C|GetcurrentStage _asglobal_value)))))
    (else
      (bind _aspuzzle_player_controller (Utilities|Casting|CastToPuzzlePlayerController (Game|GetPlayerController 0)))
      (Rendering|Material|SetTextureParameterValue (stale EventBeginPlay _returnvalue) "StageTexture" (.defaultcapture (.Value (Utilities|Map|Find (Variables|/Game/PuzzleBP/Blueprints/PuzzlePlayerController.PuzzlePlayerController_C|GetChapterMap _aspuzzle_player_controller) (Variables|/Game/Xu/Blueprints/GlobalValue.GlobalValue_C|GetcurrentChapter _asglobal_value))))))))

(fn ConstructionScript)